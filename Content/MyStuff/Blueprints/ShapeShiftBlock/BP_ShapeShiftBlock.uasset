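; BP_ShapeShiftBlock is a block that alters the third-person character's movement or health on overlap, according to its BlockState.
; Overlap asks PathManagerRef for a new path (the random check always passes as set), then applies normal, slippery, bouncy, sticky or magma behavior.
; ResetAllProperties restores default movement values, also on overlap end.
; Magma damage repeats on a Delay loop that leaving the block does not stop.
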(event OnComponentEndOverlap(BoxCollision)
  (params (OverlappedComponent :type Primitive%20Component%20Object%20Reference) (OtherActor :type Actor%20Object%20Reference) (OtherComp :type Primitive%20Component%20Object%20Reference) (OtherBodyIndex :type Integer))
  (CallFunction|ResetAllProperties OtherActor))

(event OnComponentBeginOverlap(BoxCollision)
  (params (OverlappedComponent :type Primitive%20Component%20Object%20Reference) (OtherActor :type Actor%20Object%20Reference) (OtherComp :type Primitive%20Component%20Object%20Reference) (OtherBodyIndex :type Integer) (bFromSweep :type Boolean) (SweepResult :type Hit%20Result%20Structure%20%28by%20ref%29))
  (Variables|Default|SetHasTriggeredPath true)
  (Utilities|Casting|CastToBP_ThirdPersonCharacter OtherActor)
  (if (< (Math|Random|RandomFloatinRange 0.0 0.0) 0.2)
    (bind _pathmanagerref (Variables|Default|GetPathManagerRef)
      (:then
        (Default|GenerateNewPath _pathmanagerref))
      (:else)))
  (Variables|Default|SetOtherOverlapperActor OtherActor)
  (switch Utilities|FlowControl|Switch|SwitchonBlockStates (Variables|Default|GetBlockState)
    (:NewEnumerator0
      (CallFunction|ResetAllProperties (Variables|Default|GetOtherOverlapperActor)))
    (:NewEnumerator1
      (bind _asbp_third_person_character (Utilities|Casting|CastToBP_ThirdPersonCharacter (Variables|Default|GetOtherOverlapperActor)))
      (CallFunction|ResetAllProperties (Variables|Default|GetOtherOverlapperActor))
      (Variables|/Script/Engine.CharacterMovementComponent|SetMaxWalkSpeed (Variables|/Script/Engine.Character|GetCharacterMovement _asbp_third_person_character) 8e+02)
      (Variables|/Script/Engine.CharacterMovementComponent|SetBrakingDecelerationWalking (Variables|/Script/Engine.Character|GetCharacterMovement _asbp_third_person_character) 3e+02)
      (Variables|/Script/Engine.CharacterMovementComponent|SetGroundFriction (Variables|/Script/Engine.Character|GetCharacterMovement _asbp_third_person_character) 1.0)
      (Variables|/Script/Engine.CharacterMovementComponent|SetGravityScale (Variables|/Script/Engine.Character|GetCharacterMovement _asbp_third_person_character) 5.0)
      (Pawn|Components|CharacterMovement|SetWalkableFloorAngle (Variables|/Script/Engine.Character|GetCharacterMovement _asbp_third_person_character) 0.0))
    (:NewEnumerator2
      (bind _asbp_third_person_character_2 (Utilities|Casting|CastToBP_ThirdPersonCharacter (Variables|Default|GetOtherOverlapperActor)))
      (CallFunction|ResetAllProperties (Variables|Default|GetOtherOverlapperActor))
      (Variables|/Script/Engine.MovementComponent|SetVelocity (Variables|/Script/Engine.Character|GetCharacterMovement _asbp_third_person_character_2) (+ (Variables|/Script/Engine.MovementComponent|GetVelocity (Variables|/Script/Engine.Character|GetCharacterMovement _asbp_third_person_character_2)) "0.000000,0.000000,800.000000")))
    (:NewEnumerator3
      (bind _asbp_third_person_character_3 (Utilities|Casting|CastToBP_ThirdPersonCharacter (Variables|Default|GetOtherOverlapperActor)))
      (CallFunction|ResetAllProperties (Variables|/Script/Engine.Character|GetCharacterMovement _asbp_third_person_character_3))
      (Variables|/Script/Engine.CharacterMovementComponent|SetMaxWalkSpeed (Variables|/Script/Engine.Character|GetCharacterMovement _asbp_third_person_character_3) 3e+02))
    (:NewEnumerator4
      (bind _asbp_third_person_character_4 (Utilities|Casting|CastToBP_ThirdPersonCharacter (Variables|Default|GetOtherOverlapperActor)))
      (CallFunction|ResetAllProperties (Variables|Default|GetOtherOverlapperActor))
      (Default|Damage (Variables|/Game/ThirdPerson/Blueprints/BP_ThirdPersonCharacter.BP_ThirdPersonCharacter_C|GetHealthSystem _asbp_third_person_character_4) 1e+01 :!label _label)
      (Utilities|FlowControl|Delay 1.0)
      (goto _label))))

(event EventBeginPlay)

(fn ConstructionScript)

(fn ResetAllProperties
  (params (Object :type Object%20Object%20Reference))
  (bind _asbp_third_person_character (Utilities|Casting|CastToBP_ThirdPersonCharacter Object))
  (Variables|/Script/Engine.CharacterMovementComponent|SetBrakingDecelerationWalking (Variables|/Script/Engine.Character|GetCharacterMovement _asbp_third_person_character) (Variables|DefaultValues|GetDefault%20Braking%20Deceleration%20Walking))
  (Variables|/Script/Engine.CharacterMovementComponent|SetGroundFriction (Variables|/Script/Engine.Character|GetCharacterMovement _asbp_third_person_character) (Variables|DefaultValues|GetDefault%20Ground%20Friction))
  (Variables|/Script/Engine.CharacterMovementComponent|SetGravityScale (Variables|/Script/Engine.Character|GetCharacterMovement _asbp_third_person_character) (Variables|DefaultValues|GetDefault%20Gravity%20Scale))
  (Pawn|Components|CharacterMovement|SetWalkableFloorAngle (Variables|/Script/Engine.Character|GetCharacterMovement _asbp_third_person_character) (Variables|DefaultValues|GetDefault%20Walkable%20Floor%20Angle))
  (Variables|/Script/Engine.CharacterMovementComponent|SetJumpZVelocity (Variables|/Script/Engine.Character|GetCharacterMovement _asbp_third_person_character) (Variables|DefaultValues|GetDefaultJumpVelocity))
  (Variables|/Script/Engine.CharacterMovementComponent|SetMaxWalkSpeed (Variables|/Script/Engine.Character|GetCharacterMovement _asbp_third_person_character) (Variables|DefaultValues|GetDefaultMaxWalkSpeed)))